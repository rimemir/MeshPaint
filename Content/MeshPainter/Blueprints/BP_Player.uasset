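; BP_Player is the player Blueprint for a mesh painting setup, letting the player paint whatever actor they aim at.
; Shortly after BeginPlay it caches the first BP_Capture actor in the level.
; While the Shoot axis is positive, it line traces on Visibility from the actor's location along the control rotation.
; Hits pass the actor, location and a fixed brush radius to the capture actor's PaintActor.
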(event `self.ReceiveBeginPlay`
  (`KismetSystemLibrary.Delay` 0.1)
  (bind _outactors (`GameplayStatics.GetAllActorsOfClass` "/Game/MeshPainter/Blueprints/BP_Capture.BP_Capture_C"))
  (bind _output (`|GetArrayItem` _outactors))
  (`/Engine/EditorBlueprintResources/StandardMacros.IsValid` _output
    (:`Is Valid`
      (set `self.CaptureActor` _output))))

(event `InputAxis|Shoot`
  (params (AxisValue :type "Float (single-precision)"))
  (if (> AxisValue 0.0)
    (`self.Shoot`)))

(fn `Shoot`
  (bind _returnvalue (`self.K2_GetActorLocation`))
  (bind (_outhit _returnvalue_2) (`KismetSystemLibrary.LineTraceSingle` _returnvalue (+ _returnvalue (* (`KismetMathLibrary.GetForwardVector` (`self.GetControlRotation`)) (`self.ShootDistance`))) "TraceTypeQuery1"))
  (if _returnvalue_2
    (bind (_bblockinghit _binitialoverlap _time _distance _location _impactpoint _normal _impactnormal _physmat _hitactor) (`GameplayStatics.BreakHitResult` _outhit))
    (`/Game/MeshPainter/Blueprints/BP_Capture.PaintActor` (`self.CaptureActor`) _hitactor _location 20.0)))

(fn `UserConstructionScript`)