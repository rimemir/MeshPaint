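; BP_Capture is a mesh painting helper that renders brush hits on a Character's mesh into a render target through an unwrap material.
; On BeginPlay it writes capture size and unwrap location to a global parameter collection, clears RT_Capture and creates the dynamic unwrap material.
; PaintActor temporarily swaps that material onto the mesh's first slot, passes hit location and brush radius, captures the scene, then restores the original.
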(event `self.ReceiveBeginPlay`
  (`self.InitializeParameters`
    (:`Out`
      (bind _returnvalue (`KismetMaterialLibrary.CreateDynamicMaterialInstance` "/Game/MeshPainter/Materials/M_Unwrap.M_Unwrap"))
      (set `self.UnwrapMaterial` _returnvalue))))

(fn `PaintActor`
  (params (ActorToPaint :type "Actor Object Reference") (HitLocation :type "Vector Structure") (BrushRadius :type "Float (double-precision)"))
  (bind _ascharacter (cast `Character` ActorToPaint))
  (set `self.MeshComponent` (`Character.Mesh` _ascharacter))
  (`|ExecutionSequence`
    (:`then_0`
      (set `self.OriginalMaterial` (`PrimitiveComponent.GetMaterial` (`self.MeshComponent`) 0))
      (`PrimitiveComponent.SetMaterial` (`self.MeshComponent`) 0 (`self.UnwrapMaterial`)))
    (:`then_1`
      (`MaterialInstanceDynamic.SetVectorParameterValue` (`self.UnwrapMaterial`) "HitLocation" (`KismetMathLibrary.Conv_VectorToLinearColor` (`local.HitLocation`)))
      (`MaterialInstanceDynamic.SetScalarParameterValue` (`self.UnwrapMaterial`) "BrushRadius" (`local.BrushRadius`)))
    (:`then_2`
      (`SceneCaptureComponent2D.CaptureScene` (`self.SceneCapture`))
      (`PrimitiveComponent.SetMaterial` (`self.MeshComponent`) 0 (`self.OriginalMaterial`)))))

(fn `UserConstructionScript`)